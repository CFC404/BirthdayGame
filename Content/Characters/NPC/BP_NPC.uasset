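; BP_NPC is a talkable NPC that shows an interaction prompt and steps through a list of dialogue lines.
; Its Trigger overlap with the first-person character creates and shows a WB_E prompt widget, which hides on exit or on Talk.
; Each Talk call runs DialogueSystem, which advances TalkIndex, shows that line in a reused WB_Dialogue widget with a random-pitch sound, and removes the widget once the index exceeds the array length.
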(event OnComponentBeginOverlap(trigger)
  (params (OverlappedComponent :type Primitive%20Component%20Object%20Reference) (OtherActor :type Actor%20Object%20Reference) (OtherComp :type Primitive%20Component%20Object%20Reference) (OtherBodyIndex :type Integer) (bFromSweep :type Boolean) (SweepResult :type Hit%20Result%20Structure%20%28by%20ref%29))
  (Utilities|Casting|CastToBP_FirstPersonCharacter OtherActor)
  (bind _returnvalue (UserInterface|CreateWidget "/Game/UI/WB_E.WB_E_C" (Game|GetPlayerController 0)))
  (UserInterface|Viewport|AddtoViewport _returnvalue 0)
  (Widget|SetVisibility (Variables|/Game/UI/WB_E.WB_E_C|Gettxt_e _returnvalue) "Visible"))

(event OnComponentEndOverlap(trigger)
  (params (OverlappedComponent :type Primitive%20Component%20Object%20Reference) (OtherActor :type Actor%20Object%20Reference) (OtherComp :type Primitive%20Component%20Object%20Reference) (OtherBodyIndex :type Integer))
  (Utilities|Casting|CastToBP_FirstPersonCharacter OtherActor)
  (Widget|SetVisibility (Variables|/Game/UI/WB_E.WB_E_C|Gettxt_e (stale OnComponentBeginOverlap(trigger) _returnvalue)) "Collapsed"))

(event EventBeginPlay)

(event EventTalk
  (CallFunction|DialogueSystem)
  (Widget|SetVisibility (Variables|/Game/UI/WB_E.WB_E_C|Gettxt_e (stale OnComponentBeginOverlap(trigger) _returnvalue)) "Collapsed"))

(fn ConstructionScript)

(fn DialogueSystem
  (bind _talkindex (Variables|Default|GetTalkIndex))
  (Math|Integer|IncrementInt _talkindex
    (:%20%20
      (if (<= _talkindex (Utilities|Array|Length (Variables|Default|GetDialogue)))
        (Variables|Default|GetDialogueUI
          (:then
            _)
          (:else
            (bind _returnvalue (UserInterface|CreateWidget "/Game/UI/WB_Dialogue.WB_Dialogue_C" (Game|GetPlayerController 0)))
            (bind _output_get (Variables|Default|SetDialogueUI _returnvalue))
            (UserInterface|Viewport|AddtoViewport _output_get 0)))
        (Rendering|Components|TextRender|SetText (Variables|/Game/UI/WB_Dialogue.WB_Dialogue_C|Gettxt_CarynText (Variables|Default|GetDialogueUI)) (Utilities|Text|ToText(String) (Utilities|Array|Get(acopy) (Variables|Default|GetDialogue) (Variables|Default|GetTalkIndex))))
        (Audio|PlaySound2D "/Engine/VREditor/Sounds/VR_confirm.VR_confirm" 1.0 (Math|Random|RandomFloatinRange -1e+01 1e+01) 0.0 0 0)
        (else
          (Widget|RemovefromParent (Variables|Default|GetDialogueUI)))))))