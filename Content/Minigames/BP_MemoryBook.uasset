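; BP_MemoryBook is an interactable minigame book that opens to release a polaroid.
; Sphere overlap with BP_PuzzleCharacter enables interaction and shows a WB_E prompt widget.
; Interact swaps to the open-book mesh, spawns BP_Polaroid above it, then destroys the book after a short delay.
; Each overlap begin and end adds a new widget to the viewport; leaving only collapses the prompt text from the begin event.
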(event OnComponentBeginOverlap(Sphere)
  (params (OverlappedComponent :type Primitive%20Component%20Object%20Reference) (OtherActor :type Actor%20Object%20Reference) (OtherComp :type Primitive%20Component%20Object%20Reference) (OtherBodyIndex :type Integer) (bFromSweep :type Boolean) (SweepResult :type Hit%20Result%20Structure%20%28by%20ref%29))
  (Utilities|Casting|CastToBP_PuzzleCharacter OtherActor)
  (Variables|Default|SetOverlapping true)
  (bind _returnvalue (UserInterface|CreateWidget "/Game/UI/WB_E.WB_E_C"))
  (UserInterface|Viewport|AddtoViewport _returnvalue 0)
  (Widget|SetVisibility (Variables|/Game/UI/WB_E.WB_E_C|Gettxt_e _returnvalue) "Visible"))

(event OnComponentEndOverlap(Sphere)
  (params (OverlappedComponent :type Primitive%20Component%20Object%20Reference) (OtherActor :type Actor%20Object%20Reference) (OtherComp :type Primitive%20Component%20Object%20Reference) (OtherBodyIndex :type Integer))
  (Utilities|Casting|CastToBP_PuzzleCharacter OtherActor)
  (Variables|Default|SetOverlapping false)
  (bind _returnvalue (UserInterface|CreateWidget "/Game/UI/WB_E.WB_E_C"))
  (UserInterface|Viewport|AddtoViewport _returnvalue 0)
  (Widget|SetVisibility (Variables|/Game/UI/WB_E.WB_E_C|Gettxt_e (stale OnComponentBeginOverlap(Sphere) _returnvalue)) "Collapsed"))

(event Custom|Event%20Interact
  (bind _staticmesh (Variables|Default|GetStaticMesh))
  (bind _returnvalue (Transformation|GetWorldLocation _staticmesh))
  (if (Variables|Default|GetOverlapping)
    (CallFunction|OpenBook)
    (Game|SpawnActorfromClass "/Game/Minigames/BP_Polaroid.BP_Polaroid_C" (Math|Transform|MakeTransform (Math|Vector|MakeVector (.x _returnvalue) (.y _returnvalue) (+ (.z _returnvalue) 1e+02)) "0, 0, 0" "1.000000,1.000000,1.000000") "Undefined" "MultiplyWithRoot" 0 0)
    (Utilities|FlowControl|Delay 3.0)
    (Actor|DestroyActor)))

(event EventBeginPlay)

(event Collision|EventActorBeginOverlap
  (params (OtherActor :type Actor%20Object%20Reference)))

(event EventTick
  (params (DeltaSeconds :type Float%20%28single-precision%29)))

(fn ConstructionScript)

(fn OpenBook
  (Components|StaticMesh|SetStaticMesh (Variables|Default|GetStaticMesh) "/Game/Minigames/mbopen.mbopen"))